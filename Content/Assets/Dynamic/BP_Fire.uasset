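; BP_Fire is a fireball projectile that shows effects on spawn and on impact and can damage the third-person character.
; On BeginPlay it spawns a shockwave particle at its location, tinted by its Color variable.
; On Hit it spawns an emitter at the impact point, with no template set, then casts the other actor to BP_ThirdPersonCharacter.
; Only a successful cast leads to the damage call and self-destruction.
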(event `self.ReceiveBeginPlay`
  ;[1 1 1] 파이어볼 등장시 시각 효과 생성
  (bind _returnvalue (`GameplayStatics.SpawnEmitterAtLocation` "/Game/FXVarietyPack/Particles/P_ky_shotShockwave.P_ky_shotShockwave" (`self.K2_GetActorLocation`) (`self.K2_GetActorRotation`)))
  (`ParticleSystemComponent.SetVectorParameter` _returnvalue "color" (`KismetMathLibrary.Conv_LinearColorToVector` (`self.color`))))

(event `self.ReceiveHit`
  (params (MyComp :type "PrimitiveComponent Object Reference") (Other :type "Actor Object Reference") (OtherComp :type "PrimitiveComponent Object Reference") (bSelfMoved :type Boolean) (HitLocation :type "Vector Structure") (HitNormal :type "Vector Structure") (NormalImpulse :type "Vector Structure") (Hit :type "HitResult Structure (by ref)"))
  (`GameplayStatics.SpawnEmitterAtLocation` null HitLocation)
  (bind _asbp_third_person_character (cast `/Game/ThirdPerson/Blueprints/BP_ThirdPersonCharacter` Other))
  (if (`KismetSystemLibrary.IsValid` _asbp_third_person_character)
    (`GameplayStatics.ApplyDamage` null))
  (`self.K2_DestroyActor`))

(fn `UserConstructionScript`)