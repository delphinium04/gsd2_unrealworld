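; BP_MonsterController is an AI controller that switches a monster between patrolling, chasing and attacking without a behavior tree.
; A looping timer started at BeginPlay calls Patrol, which moves to a random reachable point around the first TargetPoint found in the level.
; While IsChasing is set, Tick either calls Attack on the controlled pawn when CanAttack is true or moves toward TargetActor.
; The file never sets those state variables or pauses the patrol timer.
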(event `self.ReceiveBeginPlay`
  ; 시작시 순찰
  (`KismetSystemLibrary.K2_SetTimer` null "Patrol" 5.0 true))

(event `self.ReceiveTick`
  (params (DeltaSeconds :type "Float (single-precision)"))
  ; 몬스터 행동 로직
  (if (`self.IsChasing`)
    (if (`self.CanAttack`)
      (bind _asbp_boss_monster (cast `` (`self.K2_GetPawn`)))
      (`self.Attack` _asbp_boss_monster)
      (else
        (`|AIMoveTo` null (0.0 0.0 0.0) (`self.TargetActor`) 30.0)))))

(fn `Patrol`
  (bind _outactors (`GameplayStatics.GetAllActorsOfClass` "/Script/Engine.TargetPoint"))
  (`self.MoveToLocation` (`NavigationSystemV1.K2_GetRandomReachablePointInRadius` (`self.K2_GetActorLocation` (`|GetArrayItem` _outactors)) 800.0 null null) -1.0 true true false true null))

(fn `UserConstructionScript`)