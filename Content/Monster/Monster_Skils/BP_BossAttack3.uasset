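; BP_BossAttack3 is a boss attack projectile that damages the player on impact.
; It starts with ProjectileEffect active and ShootParticle off, and the ShootProjectile event swaps the two effects.
; On any hit it spawns an impact emitter, applies fixed damage if the other actor is the PlayerCharacter, then destroys itself.
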(event `self.ReceiveBeginPlay`
  (`ActorComponent.Activate` (`self.ProjectileEffect`) false)
  (`ActorComponent.Deactivate` (`self.ShootParticle`)))

(event `self.ShootProjectile`
  (`ActorComponent.Deactivate` (`self.ProjectileEffect`))
  (`ActorComponent.Activate` (`self.ShootParticle`) false))

(event `self.ReceiveHit`
  (params (MyComp :type "PrimitiveComponent Object Reference") (Other :type "Actor Object Reference") (OtherComp :type "PrimitiveComponent Object Reference") (bSelfMoved :type Boolean) (HitLocation :type "Vector Structure") (HitNormal :type "Vector Structure") (NormalImpulse :type "Vector Structure") (Hit :type "HitResult Structure (by ref)"))
  (`GameplayStatics.SpawnEmitterAtLocation` "/Game/Monster/Monster_Skils/Boss_Skil_Particle/Boss_Attack3_hit.Boss_Attack3_hit" HitLocation)
  (bind _asplayer_character (cast `PlayerCharacter` Other)
    (:`then`
      (`GameplayStatics.ApplyDamage` _asplayer_character 5.0))
    (:`CastFailed`
      _))
  (`self.K2_DestroyActor`))

(fn `UserConstructionScript`)