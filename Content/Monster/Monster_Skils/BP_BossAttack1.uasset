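; BP_BossAttack1 is a boss attack projectile that flies straight, then partially homes in on its TargetActor.
; Tick drives ProjectileMovement velocity along the initial direction until StartHomingTime, then uses an even blend of that direction and the direction to the target.
; Hits spawn an impact emitter, damage only player characters and destroy the projectile.
; Otherwise, a delay started in the homing phase makes it burst and self-destroy.
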(event `self.ReceiveTick`
  (params (DeltaSeconds :type "Float (single-precision)"))
  (bind _targetactor (`self.TargetActor`))
  (bind _projectilemovement (`self.ProjectileMovement`))
  (bind _initaldirection (`self.InitalDirection`))
  (bind _initialspeed (`ProjectileMovementComponent.InitialSpeed` _projectilemovement))
  (`/Engine/EditorBlueprintResources/StandardMacros.IsValid` _targetactor
    (:`Is Valid`
      (bind _output_get (set `self.ElapsedTime` (+ (`self.ElapsedTime`) DeltaSeconds)))
      (if (< _output_get (`self.StartHomingTime`))
        (set `MovementComponent.Velocity` (* _initialspeed _initaldirection) _projectilemovement)
        (else
          (set `MovementComponent.Velocity` (* _initialspeed (`KismetMathLibrary.VLerp` (`KismetMathLibrary.Normal` (- (`self.K2_GetActorLocation` _targetactor) (`self.K2_GetActorLocation`))) _initaldirection 0.5)) _projectilemovement)
          (`KismetSystemLibrary.Delay` 5.0)
          (`GameplayStatics.SpawnEmitterAtLocation` "/Game/Monster/Monster_Skils/Boss_Skil_Particle/Boss_Attack1_hit.Boss_Attack1_hit" (`self.K2_GetActorLocation`))
          (`self.K2_DestroyActor`))))))

(event `self.ReceiveHit`
  (params (MyComp :type "PrimitiveComponent Object Reference") (Other :type "Actor Object Reference") (OtherComp :type "PrimitiveComponent Object Reference") (bSelfMoved :type Boolean) (HitLocation :type "Vector Structure") (HitNormal :type "Vector Structure") (NormalImpulse :type "Vector Structure") (Hit :type "HitResult Structure (by ref)"))
  (`GameplayStatics.SpawnEmitterAtLocation` "/Game/Monster/Monster_Skils/Boss_Skil_Particle/Boss_Attack1_hit.Boss_Attack1_hit" HitLocation)
  (bind _asplayer_character (cast `PlayerCharacter` Other)
    (:`then`
      (`GameplayStatics.ApplyDamage` _asplayer_character 5.0))
    (:`CastFailed`
      _))
  (`self.K2_DestroyActor`))

(fn `UserConstructionScript`)