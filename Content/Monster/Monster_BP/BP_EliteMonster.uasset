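; Elite monster Blueprint that deals melee damage to the player through collision components on its left and right arms.
; BeginPlay disables both arm colliders, and nothing in this graph re-enables them.
; When either arm overlaps a PlayerCharacter, it applies AttackDamage only if CanCloseDealDamage is true.
; Debug strings report each overlap and whether damage is dealt.
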(event `self.ReceiveBeginPlay`
  ; 손 콜리전 시작시 전부 비활성화
  (`PrimitiveComponent.SetCollisionEnabled` (`self.왼쪽팔`) "NoCollision")
  (`PrimitiveComponent.SetCollisionEnabled` (`self.오른쪽팔`) "NoCollision"))

(event `self.오른쪽팔.OnComponentBeginOverlap`
  (params (OverlappedComponent :type "PrimitiveComponent Object Reference") (OtherActor :type "Actor Object Reference") (OtherComp :type "PrimitiveComponent Object Reference") (OtherBodyIndex :type Integer) (bFromSweep :type Boolean) (SweepResult :type "HitResult Structure (by ref)"))
  (bind _asplayer_character (cast `PlayerCharacter` OtherActor))
  (`KismetSystemLibrary.PrintString` "오른팔과 오버랩됨!")
  (if (`self.bCanCloseDealDamage`)
    (`GameplayStatics.ApplyDamage` _asplayer_character (`self.AttackDamage`))
    (`KismetSystemLibrary.PrintString` "데미지 전달")
    (else
      (`KismetSystemLibrary.PrintString` "어택불가"))))

(event `self.왼쪽팔.OnComponentBeginOverlap`
  (params (OverlappedComponent :type "PrimitiveComponent Object Reference") (OtherActor :type "Actor Object Reference") (OtherComp :type "PrimitiveComponent Object Reference") (OtherBodyIndex :type Integer) (bFromSweep :type Boolean) (SweepResult :type "HitResult Structure (by ref)"))
  (bind _asplayer_character (cast `PlayerCharacter` OtherActor))
  (`KismetSystemLibrary.PrintString` "왼쪽팔과 오버랩됨!")
  (if (`self.bCanCloseDealDamage`)
    (`GameplayStatics.ApplyDamage` _asplayer_character (`self.AttackDamage`))
    (`KismetSystemLibrary.PrintString` "데미지 전달")
    (else
      (`KismetSystemLibrary.PrintString` "어택불가"))))

(fn `UserConstructionScript`)