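; Puzzle actor that is solved when its left and right areas hold equal counts of overlapping target actors, optionally also matching a target number.
; BeginPlay and every begin or end overlap on either area recount both sides, adding the player when IncludePlayer is set.
; CheckPuzzleEnd then compares the counts and broadcasts OnPuzzleSolved through a DoOnce, so it fires a single time.
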(event `self.ReceiveBeginPlay`
  (`parent.ReceiveBeginPlay`)
  (`self.SetDefaultCount`))

(event `self.LeftArea.OnComponentBeginOverlap`
  (params (OverlappedComponent :type "PrimitiveComponent Object Reference") (OtherActor :type "Actor Object Reference") (OtherComp :type "PrimitiveComponent Object Reference") (OtherBodyIndex :type Integer) (bFromSweep :type Boolean) (SweepResult :type "HitResult Structure (by ref)"))
  (`self.SetDefaultCount` :!label _label))

(event `self.RightArea.OnComponentBeginOverlap`
  (params (OverlappedComponent :type "PrimitiveComponent Object Reference") (OtherActor :type "Actor Object Reference") (OtherComp :type "PrimitiveComponent Object Reference") (OtherBodyIndex :type Integer) (bFromSweep :type Boolean) (SweepResult :type "HitResult Structure (by ref)"))
  (goto _label))

(event `self.LeftArea.OnComponentEndOverlap`
  (params (OverlappedComponent :type "PrimitiveComponent Object Reference") (OtherActor :type "Actor Object Reference") (OtherComp :type "PrimitiveComponent Object Reference") (OtherBodyIndex :type Integer))
  (goto _label))

(event `self.RightArea.OnComponentEndOverlap`
  (params (OverlappedComponent :type "PrimitiveComponent Object Reference") (OtherActor :type "Actor Object Reference") (OtherComp :type "PrimitiveComponent Object Reference") (OtherBodyIndex :type Integer))
  (goto _label))

(fn `CheckPuzzleEnd`
  (bind _rightcount (`self.RightCount`))
  (if (== _rightcount (`self.LeftCount`))
    (if (or (and (`self.bHasTargetNumber`) (== (`self.TargetNumber`) _rightcount)) (not (`self.bHasTargetNumber`)))
      (`/Engine/EditorBlueprintResources/StandardMacros.DoOnce` false
        (:`Completed`
          (`self.BroadcastOnPuzzleSolved`))))))

(fn `SetDefaultCount`
  (locals (LCount :type Integer :default 0) (RCount :type Integer))
  (bind _leftarea (`self.LeftArea`))
  (bind _rightarea (`self.RightArea`))
  (set `local.LCount` (`self.GetOverlapCount` _leftarea))
  (if (`self.IsPlayerOverlap` _leftarea)
    (`/Engine/EditorBlueprintResources/StandardMacros.IncrementInt` (`local.LCount`)
      (:`  `
        _)))
  (set `self.LeftCount` (`local.LCount`))
  (set `local.RCount` (`self.GetOverlapCount` _rightarea))
  (if (`self.IsPlayerOverlap` _rightarea)
    (`/Engine/EditorBlueprintResources/StandardMacros.IncrementInt` (`local.RCount`)
      (:`  `
        _)))
  (set `self.RightCount` (`local.RCount`))
  (`self.CheckPuzzleEnd`))

(fn `UserConstructionScript`
  (`parent.UserConstructionScript`))