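; Puzzle actor that activates a Target actor while its pressure plate is pressed and is solved once that Target moves.
; Target starts inactive; pressing the plate records its location and activates it, while releasing deactivates it only if it has not moved.
; Tick compares the Target against the recorded location and, on the first noticeable displacement, unbinds the plate and broadcasts puzzle solved through a DoOnce.
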(event `self.ReceiveBeginPlay`
  (bind _target (`self.Target`))
  (`parent.ReceiveBeginPlay`)
  (set `self.TargetLocation` (`self.K2_GetActorLocation` _target))
  (`ActorBlueprintLibraryExtension.ActorSetActive` _target false)
  (add `InteractableActor.OnInteracted` (`self.Plate`) (delegate `Pressed`)))

(event `Pressed`
  (params (Caller :type "InteractableActor Object Reference"))
  (bind _target (`self.Target`))
  (if (`/Game/Puzzles/Blueprints/BP_PuzzlePlate.bIsPressed` (`self.Plate`))
    (set `self.TargetLocation` (`self.K2_GetActorLocation` _target))
    (`ActorBlueprintLibraryExtension.ActorSetActive` _target)
    (elif (== (`self.TargetLocation`) (`self.K2_GetActorLocation` (`self.Target`)) :`ErrorTolerance` 0.1)
      (`ActorBlueprintLibraryExtension.ActorSetActive` (`self.Target`) false))))

(event `self.ReceiveTick`
  (params (DeltaSeconds :type "Float (single-precision)"))
  (`parent.ReceiveTick` DeltaSeconds)
  (if (not (== (`self.TargetLocation`) (`self.K2_GetActorLocation` (`self.Target`)) :`ErrorTolerance` 1.0))
    (`/Engine/EditorBlueprintResources/StandardMacros.DoOnce` false
      (:`Completed`
        (clear `InteractableActor.OnInteracted` (`self.Plate`))
        (`self.BroadcastOnPuzzleSolved`)))))

(fn `UserConstructionScript`
  (`parent.UserConstructionScript`))