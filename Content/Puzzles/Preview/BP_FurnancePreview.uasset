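; Furnace puzzle controller that counts interactions with an array of furnace actors and broadcasts OnPuzzleSolved once the count reaches the array length.
; It binds each furnace's OnInteracted; with IsOrdering set, a furnace out of array order resets the puzzle, otherwise any interaction counts.
; Interacting with any OtherActorsNeedToReset actor also resets the counters and all linked actors.
; On solve, it unbinds all interaction events.
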(event `self.ReceiveBeginPlay`
  (`parent.ReceiveBeginPlay`)
  (for _array_element (`self.Furnance`)
    (add `InteractableActor.OnInteracted` _array_element (delegate `CheckFurnance`)))
  (for _array_element_2 (`self.OtherActorsNeedToReset`)
    (add `InteractableActor.OnInteracted` _array_element_2 (delegate `ResetAll`))))

(event `ResetAll`
  (params (Caller :type "InteractableActor Object Reference"))
  (`self.Reset`))

(event `CheckFurnance`
  (params (Caller :type "InteractableActor Object Reference"))
  (if (== Caller (`|GetArrayItem` (`self.Furnance`) (`self.CurrentCount`)))
    (`/Engine/EditorBlueprintResources/StandardMacros.IncrementInt` (`self.OrderCount`) :!label _label
      (:`  `
        (`/Engine/EditorBlueprintResources/StandardMacros.IncrementInt` (`self.CurrentCount`)
          (:`  `
            (`self.CheckClear`)))))
    (elif (`self.bIsOrdering`)
      (`self.Reset`)
      (else
        (goto _label)))))

(fn `CheckClear`
  (if (>= (`self.CurrentCount`) (`KismetArrayLibrary.Array_Length` (`self.Furnance`)))
    (`/Engine/EditorBlueprintResources/StandardMacros.DoOnce` false
      (:`Completed`
        (for _array_element (`self.Furnance`)
          (clear `InteractableActor.OnInteracted` _array_element))
        (for _array_element_2 (`self.OtherActorsNeedToReset`)
          (clear `InteractableActor.OnInteracted` _array_element_2))
        (`self.BroadcastOnPuzzleSolved`)))))

(fn `Reset`
  (set `self.OrderCount` 0)
  (set `self.CurrentCount` 0)
  (for _array_element (`self.Furnance`)
    (`InteractableActor.Reset` _array_element))
  (for _array_element_2 (`self.OtherActorsNeedToReset`)
    (`InteractableActor.Reset` _array_element_2)))

(fn `UserConstructionScript`
  (`parent.UserConstructionScript`))