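; BP_TorchPreview is a torch order puzzle that is solved by interacting with its Torches in array order.
; On BeginPlay it binds each torch's OnInteracted event to a check that advances CurrentIndex on a match and counts every interaction.
; Completing the sequence broadcasts OnPuzzleSolved once and unbinds the torches.
; Otherwise, once the interaction count reaches the array length, all torches and counters reset, so mistakes are not punished immediately.
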(event `self.ReceiveBeginPlay`
  (`parent.ReceiveBeginPlay`)
  (for _array_element (`self.Torches`)
    (add `InteractableActor.OnInteracted` _array_element (delegate `CheckInteractable`))))

(event `CheckInteractable`
  (params (Caller :type "InteractableActor Object Reference"))
  (`KismetSystemLibrary.PrintString` (`KismetSystemLibrary.GetDisplayName` Caller))
  (if (== Caller (`|GetArrayItem` (`self.Torches`) (`self.CurrentIndex`)))
    (`/Engine/EditorBlueprintResources/StandardMacros.IncrementInt` (`self.CurrentIndex`)
      (:`  `
        _)))
  (`/Engine/EditorBlueprintResources/StandardMacros.IncrementInt` (`self.Count`)
    (:`  `
      (if (`self.GreatEqualThanLength` (`self.CurrentIndex`))
        (`self.PuzzleSolved`)
        (elif (`self.GreatEqualThanLength` (`self.Count`))
          (`self.ResetTorches`))))))

(fn `PuzzleSolved`
  (`/Engine/EditorBlueprintResources/StandardMacros.DoOnce` false
    (:`Completed`
      (`self.BroadcastOnPuzzleSolved`)
      (for _array_element (`self.Torches`)
        (clear `InteractableActor.OnInteracted` _array_element)))))

(fn `ResetTorches`
  (for _array_element (`self.Torches`)
    (`InteractableActor.Reset` _array_element))
  (set `self.CurrentIndex` 0)
  (set `self.Count` 0))

(fn `UserConstructionScript`
  (`parent.UserConstructionScript`))