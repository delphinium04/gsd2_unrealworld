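; Level puzzle actor for PuzzleTest1 that tracks whether every cube checker holds at least one cube.
; On BeginPlay it binds to each checker's CountUpdated event, rechecking all counts on every change.
; The result toggles the ClearEffects Niagara effects, and both outcomes fire OnPuzzleSolved.
; Solved is only ever cleared here, never set true, and ResetPuzzle is an empty stub.
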(event `self.ReceiveBeginPlay`
  (`parent.ReceiveBeginPlay`)
  (for _array_element (`self.BP_CubeChecker`)
    (add `/Game/Puzzles/Level/PuzzleTest1/BP_TestCheckCube.CountUpdated` _array_element (delegate `Box Added`))))

(event `Box Added`
  (`KismetSystemLibrary.PrintString` "Event Called")
  (`self.CheckPuzzleState`))

(event `self.ReceiveTick`
  (params (DeltaSeconds :type "Float (single-precision)"))
  (`parent.ReceiveTick` DeltaSeconds))

(fn `CheckPuzzleState`
  (locals (Solved :type Boolean :default true))
  (for _array_element (`self.BP_CubeChecker`)
    (if (< (`/Game/Puzzles/Level/PuzzleTest1/BP_TestCheckCube.CubeCount` _array_element) 1)
      (set `local.Solved` false)
      (`KismetSystemLibrary.PrintString` "Nope")
      (break)))
  (if (`local.Solved`)
    (`self.Solve`)
    (`KismetSystemLibrary.PrintString` "Puzzle 1 Solved")
    (else
      (`self.DeSolve`))))

(fn `DeSolve`
  (`self.OnPuzzleSolved`)
  (for _array_element (`self.ClearEffects`)
    (`ActorComponent.Deactivate` (`NiagaraActor.NiagaraComponent` _array_element))))

(fn `ResetPuzzle`)

(fn `Solve`
  (`self.OnPuzzleSolved`)
  (for _array_element (`self.ClearEffects`)
    (`ActorComponent.Activate` (`NiagaraActor.NiagaraComponent` _array_element) false)
    (`KismetSystemLibrary.PrintString` "Effec tOn")))

(fn `UserConstructionScript`
  (`parent.UserConstructionScript`))