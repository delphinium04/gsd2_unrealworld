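; BP_TestCheckCube is a puzzle check zone that counts BP_TestCube actors of a matching Type inside its Box.
; Box begin and end overlaps raise or lower CubeCount, then broadcast CountUpdated and refresh the effect.
; The referenced VFX's Niagara component, if valid, stays active while at least one matching cube is inside.
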(event `self.Box.OnComponentBeginOverlap`
  (params (OverlappedComponent :type "PrimitiveComponent Object Reference") (OtherActor :type "Actor Object Reference") (OtherComp :type "PrimitiveComponent Object Reference") (OtherBodyIndex :type Integer) (bFromSweep :type Boolean) (SweepResult :type "HitResult Structure (by ref)"))
  (bind _asbp_test_cube (cast `/Game/Puzzles/Level/PuzzleTest1/BP_TestCube` OtherActor))
  (if (`|EnumEquality` (`/Game/Puzzles/Level/PuzzleTest1/BP_TestCube.Type` _asbp_test_cube) (`self.Type`))
    (set `self.CubeCount` (+ (`self.CubeCount`) 1))
    (`self.CountUpdated`)
    (`self.UpdateNiagaraEffect`)))

(event `self.Box.OnComponentEndOverlap`
  (params (OverlappedComponent :type "PrimitiveComponent Object Reference") (OtherActor :type "Actor Object Reference") (OtherComp :type "PrimitiveComponent Object Reference") (OtherBodyIndex :type Integer))
  (bind _asbp_test_cube (cast `/Game/Puzzles/Level/PuzzleTest1/BP_TestCube` OtherActor))
  (if (`|EnumEquality` (`/Game/Puzzles/Level/PuzzleTest1/BP_TestCube.Type` _asbp_test_cube) (`self.Type`))
    (set `self.CubeCount` (+ (`self.CubeCount`) -1))
    (`self.CountUpdated`)
    (`self.UpdateNiagaraEffect`)))

(fn `UpdateNiagaraEffect`
  (bind _vfx (`self.VFX`))
  (`/Engine/EditorBlueprintResources/StandardMacros.IsValid` _vfx
    (:`Is Valid`
      (`ActorComponent.SetActive` (`NiagaraActor.NiagaraComponent` _vfx) (> (`self.CubeCount`) 0) false))))

(fn `UserConstructionScript`)