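; BP_StandArea is a puzzle stand spot that detects when the player character steps into its box.
; On overlap by BP_ThirdPersonCharacter_Child it disables further overlap events and fires the OnBeginOverlapPlayer dispatcher, passing itself.
; ResetEffect re-arms the box and leaves the referenced Niagara effect active only if FirstNode is set.
; ActivateEffect switches that effect on separately, without touching the box.
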(event `self.ReceiveBeginPlay`)

(event `self.Box.OnComponentBeginOverlap`
  (params (OverlappedComponent :type "PrimitiveComponent Object Reference") (OtherActor :type "Actor Object Reference") (OtherComp :type "PrimitiveComponent Object Reference") (OtherBodyIndex :type Integer) (bFromSweep :type Boolean) (SweepResult :type "HitResult Structure (by ref)"))
  (cast `/Game/Puzzles/Level/BP_ThirdPersonCharacter_Child` OtherActor)
  (set `PrimitiveComponent.bGenerateOverlapEvents` false (`self.Box`))
  (`self.OnBeginOverlapPlayer` self))

(fn `ActivateEffect`
  (`ActorComponent.Activate` (`NiagaraActor.NiagaraComponent` (`self.Effect`)) false))

(fn `ResetEffect`
  (locals (OnOverlapWithPlayer :type Boolean))
  (bind _niagaracomponent (`NiagaraActor.NiagaraComponent` (`self.Effect`)))
  (set `PrimitiveComponent.bGenerateOverlapEvents` true (`self.Box`))
  (if (`self.bFirstNode`)
    (`ActorComponent.Activate` _niagaracomponent false)
    (else
      (`ActorComponent.Deactivate` _niagaracomponent))))

(fn `UserConstructionScript`)