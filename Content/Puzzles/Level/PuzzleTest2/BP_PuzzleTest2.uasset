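; BP_PuzzleTest2 is a sequence puzzle solved by the player overlapping StandAreas in order.
; It flags the first area, binds each area's overlap event and tracks progress, activating the next area's effect on correct steps and resetting all on mistakes.
; Solving unbinds the areas, activates all their effects and activates a Niagara effect, whose color Tick randomizes every frame.
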(event `self.ReceiveBeginPlay`
  (`parent.ReceiveBeginPlay`)
  (set `/Game/Puzzles/Level/PuzzleTest2/BP_StandArea.bFirstNode` true (`|GetArrayItem` (`self.StandAreas`)))
  (for _array_element (`self.StandAreas`)
    (add `/Game/Puzzles/Level/PuzzleTest2/BP_StandArea.OnBeginOverlapPlayer` _array_element (delegate `OnOverlapBegin`))
    (`/Game/Puzzles/Level/PuzzleTest2/BP_StandArea.ResetEffect` _array_element)))

(event `OnOverlapBegin`
  (params (`Stand Area` :type "/Game/Puzzles/Level/PuzzleTest2/BP_StandArea Object Reference"))
  (bind _standareas (`self.StandAreas`))
  (if (== (`/Game/Puzzles/Level/PuzzleTest2/BP_StandArea.Order` `Stand Area`) (`self.CurrentLevel`))
    (bind _output_get (set `self.CurrentLevel` (+ (`self.CurrentLevel`) 1)))
    (if (>= _output_get (`KismetArrayLibrary.Array_Length` _standareas))
      (`self.Solve`)
      (else
        (`/Game/Puzzles/Level/PuzzleTest2/BP_StandArea.ActivateEffect` (`|GetArrayItem` _standareas (`self.CurrentLevel`)))))
    (else
      (set `self.CurrentLevel` 0)
      (for _array_element (`self.StandAreas`)
        (`/Game/Puzzles/Level/PuzzleTest2/BP_StandArea.ResetEffect` _array_element)))))

(event `self.ReceiveTick`
  (params (DeltaSeconds :type "Float (single-precision)"))
  (`parent.ReceiveTick` DeltaSeconds)
  (`NiagaraComponent.SetVariableLinearColor` (`NiagaraActor.NiagaraComponent` (`self.Niagara`)) "UserColor" (make `LinearColor` (`KismetMathLibrary.RandomFloat`) (`KismetMathLibrary.RandomFloat`) (`KismetMathLibrary.RandomFloat`) 1.0)))

(fn `Solve`
  (locals (Temp :type "/Game/Puzzles/Level/PuzzleTest2/BP_StandArea Object Reference"))
  (`ActorComponent.Activate` (`NiagaraActor.NiagaraComponent` (`self.Niagara`)) false)
  (for _array_element (`self.StandAreas`)
    (clear `/Game/Puzzles/Level/PuzzleTest2/BP_StandArea.OnBeginOverlapPlayer` _array_element)
    (`/Game/Puzzles/Level/PuzzleTest2/BP_StandArea.ActivateEffect` _array_element)))

(fn `UserConstructionScript`
  (`parent.UserConstructionScript`))