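; Base Blueprint for puzzle interactables that shows a widget prompt when a character comes within range of a grabbable object.
; The widget starts hidden, and a sphere overlap reveals it only when IsGrabbable is set and the actor has a CharacterMovementComponent.
; On reveal it rotates once to face the player camera rather than tracking it continuously, and hides again when any overlap ends.
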(event `self.ReceiveBeginPlay`
  (`SceneComponent.SetVisibility` (`self.Widget`) false false))

(event `self.SphereComponent.OnComponentBeginOverlap`
  (params (OverlappedComponent :type "PrimitiveComponent Object Reference") (OtherActor :type "Actor Object Reference") (OtherComp :type "PrimitiveComponent Object Reference") (OtherBodyIndex :type Integer) (bFromSweep :type Boolean) (SweepResult :type "HitResult Structure (by ref)"))
  (bind _widget (`self.Widget`))
  (if (and (`self.bIsGrabbable`) (`KismetSystemLibrary.IsValid` (`self.GetComponentByClass` OtherActor "/Script/Engine.CharacterMovementComponent")))
    (`SceneComponent.K2_SetWorldRotation` _widget (`KismetMathLibrary.FindLookAtRotation` (`SceneComponent.K2_GetComponentLocation` _widget) (`SceneComponent.K2_GetComponentLocation` (`Actor.RootComponent` (`GameplayStatics.GetPlayerCameraManager` 0)))) false false)
    (`SceneComponent.SetVisibility` _widget true false)))

(event `self.SphereComponent.OnComponentEndOverlap`
  (params (OverlappedComponent :type "PrimitiveComponent Object Reference") (OtherActor :type "Actor Object Reference") (OtherComp :type "PrimitiveComponent Object Reference") (OtherBodyIndex :type Integer))
  (`SceneComponent.SetVisibility` (`self.Widget`) false false))

(fn `UserConstructionScript`)