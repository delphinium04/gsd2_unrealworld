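; BP_PuzzleFurnance is an interactable puzzle furnace that lights a small Niagara fire when activated.
; On BeginPlay, ConstantOn sets both the initial fire state and IsOn.
; OnInteract calls TorchEvent, which on the first use lights the fire, sets Interacted and broadcasts OnInteracted.
; OnReset turns the fire off regardless of ConstantOn and clears Interacted, leaving IsOn untouched.
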(event `self.ReceiveBeginPlay`
  (`parent.ReceiveBeginPlay`)
  (`ActorComponent.SetActive` (`self.NS_Fire_Small_Simple`) (`self.bConstantOn`) false)
  (set `self.bIsOn` (`self.bConstantOn`)))

(event `self.OnInteract`
  (`self.TorchEvent`))

(event `self.OnReset`
  (`ActorComponent.SetActive` (`self.NS_Fire_Small_Simple`) false false)
  (set `self.bInteracted` false))

(fn `TorchEvent`
  (if (not (`self.bInteracted`))
    (`ActorComponent.SetActive` (`self.NS_Fire_Small_Simple`) true false)
    (set `self.bInteracted` true)
    (`self.BroadcastOnInteracted`)))

(fn `UserConstructionScript`
  (`parent.UserConstructionScript`))