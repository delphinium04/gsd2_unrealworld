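; BP_PuzzleTorch is a puzzle torch that exchanges fire with BP_PuzzleFurnance actors it touches.
; On sphere overlap, a burning furnace lights the torch, while a lit torch calls TorchEvent on an unlit furnace.
; SetFire stores the lit state, toggles the NS effect's visibility and restarts the timer on temporal torches.
; Tick counts that timer down and extinguishes the torch through a resettable DoOnce once it expires.
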(event `self.ReceiveBeginPlay`
  (`parent.ReceiveBeginPlay`)
  (`SceneComponent.SetVisibility` (`self.NS`) false false))

(event `self.ReceiveTick`
  (params (DeltaSeconds :type "Float (single-precision)"))
  (if (`self.bIsTemporal`)
    (set `self.Timer` (- (`self.Timer`) DeltaSeconds))
    (if (== (`self.bIsOn`) (< (`self.Timer`) -0.1))
      (`/Engine/EditorBlueprintResources/StandardMacros.DoOnce` false :!label _label
        (:`Completed`
          (`self.SetFire` false)))
      (else
        (goto _label :!via `Reset`)))))

(event `self.SphereComponent.OnComponentBeginOverlap`
  (params (OverlappedComponent :type "PrimitiveComponent Object Reference") (OtherActor :type "Actor Object Reference") (OtherComp :type "PrimitiveComponent Object Reference") (OtherBodyIndex :type Integer) (bFromSweep :type Boolean) (SweepResult :type "HitResult Structure (by ref)"))
  (bind _asbp_puzzle_furnance (cast `/Game/Puzzles/Blueprints/BP_PuzzleFurnance` OtherActor))
  (if (`/Game/Puzzles/Blueprints/BP_PuzzleFurnance.bIsOn` _asbp_puzzle_furnance)
    (`self.SetFire` true)
    (elif (`self.bIsOn`)
      (`/Game/Puzzles/Blueprints/BP_PuzzleFurnance.TorchEvent` _asbp_puzzle_furnance))))

(fn `SetFire`
  (params (enable :type Boolean))
  (bind _output_get (set `self.bIsOn` enable))
  (`SceneComponent.SetVisibility` (`self.NS`) _output_get false)
  (if (`self.bIsTemporal`)
    (set `self.Timer` (`self.FIRE_TIMER`))))

(fn `UserConstructionScript`
  (`parent.UserConstructionScript`))