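; Puzzle pressure plate that sinks when an actor of an allowed class rests on it and rises when none remain.
; Box overlaps check actors against InteractableClassType, toggle IsPressed and broadcast OnInteracted on each change.
; On release it counts remaining matching overlaps, so the plate stays pressed until the count is zero.
; Tick eases the plate vertically toward its start or lowered position, scaled by delta time.
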(event `self.ReceiveBeginPlay`
  (`parent.ReceiveBeginPlay`)
  (bind _output_get (set `self.StartPosition` (`self.K2_GetActorLocation`)))
  (set `self.EndPosition` (- _output_get (0.0 0.0 10.0))))

(event `self.ReceiveTick`
  (params (DeltaSeconds :type "Float (single-precision)"))
  (`parent.ReceiveTick` DeltaSeconds)
  (if (`self.bIsPressed`)
    (set `self.DeltaPos` (- (`self.EndPosition`) (`self.K2_GetActorLocation`)))
    (else
      (set `self.DeltaPos` (- (`self.StartPosition`) (`self.K2_GetActorLocation`)))))
  (`self.K2_AddActorLocalOffset` (* (`self.DeltaPos`) (`KismetMathLibrary.MakeVector` 0.0 0.0 DeltaSeconds))))

(event `self.Box.OnComponentBeginOverlap`
  (params (OverlappedComponent :type "PrimitiveComponent Object Reference") (OtherActor :type "Actor Object Reference") (OtherComp :type "PrimitiveComponent Object Reference") (OtherBodyIndex :type Integer) (bFromSweep :type Boolean) (SweepResult :type "HitResult Structure (by ref)"))
  (`self.OnPlatePressed` OtherActor))

(event `self.Box.OnComponentEndOverlap`
  (params (OverlappedComponent :type "PrimitiveComponent Object Reference") (OtherActor :type "Actor Object Reference") (OtherComp :type "PrimitiveComponent Object Reference") (OtherBodyIndex :type Integer))
  (`self.OnOverlapExited`))

(fn `OnOverlapExited`
  (locals (OverlapCount :type Integer))
  (if (`self.bIsPressed`)
    (for _array_element (`self.InteractableClassType`)
      (set `local.OverlapCount` (+ (`local.OverlapCount`) (`KismetArrayLibrary.Array_Length` (`PrimitiveComponent.GetOverlappingActors` (`self.Box`) _array_element)))))
    (if (== (`local.OverlapCount`) 0)
      (set `self.bIsPressed` false)
      (`self.BroadcastOnInteracted`))))

(fn `OnPlatePressed`
  (params (Object :type "Object Object Reference"))
  (locals (Isbreak :type Boolean))
  (if (not (`self.bIsPressed`))
    (set `local.Isbreak` false)
    (for _array_element (`self.InteractableClassType`)
      (if (`GameplayStatics.ObjectIsA` Object _array_element)
        (set `local.Isbreak` true)
        (break)))
    (if (`local.Isbreak`)
      (set `self.bIsPressed` true)
      (`self.BroadcastOnInteracted`))))

(fn `UserConstructionScript`
  (`parent.UserConstructionScript`))