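; Pressure plate for a Stage 1 puzzle that reacts to the player character standing on it.
; The Box trigger sets the pressed state when a player character enters, clears it when none remain, and broadcasts OnInteracted on each change.
; Tick eases the plate vertically between its start position and a slightly lowered position, moving by a delta-time-scaled share of the remaining distance.
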(event `self.ReceiveBeginPlay`
  (`parent.ReceiveBeginPlay`)
  (bind _output_get (set `self.StartPosition` (`self.K2_GetActorLocation`)))
  (set `self.EndPosition` (- _output_get (0.0 0.0 10.0))))

(event `self.ReceiveTick`
  (params (DeltaSeconds :type "Float (single-precision)"))
  (`parent.ReceiveTick` DeltaSeconds)
  (if (`self.bIsPressed`)
    (set `self.DeltaPos` (- (`self.EndPosition`) (`self.K2_GetActorLocation`)))
    (else
      (set `self.DeltaPos` (- (`self.StartPosition`) (`self.K2_GetActorLocation`)))))
  (`self.K2_AddActorLocalOffset` (* (`self.DeltaPos`) (`KismetMathLibrary.MakeVector` 0.0 0.0 DeltaSeconds))))

(event `self.Box.OnComponentBeginOverlap`
  (params (OverlappedComponent :type "PrimitiveComponent Object Reference") (OtherActor :type "Actor Object Reference") (OtherComp :type "PrimitiveComponent Object Reference") (OtherBodyIndex :type Integer) (bFromSweep :type Boolean) (SweepResult :type "HitResult Structure (by ref)"))
  (if (not (`self.bIsPressed`))
    (cast `/Game/ThirdPerson/Blueprints/BP_ThirdPersonCharacter` OtherActor)
    (set `self.bIsPressed` true)
    (`self.BroadcastOnInteracted`)))

(event `self.Box.OnComponentEndOverlap`
  (params (OverlappedComponent :type "PrimitiveComponent Object Reference") (OtherActor :type "Actor Object Reference") (OtherComp :type "PrimitiveComponent Object Reference") (OtherBodyIndex :type Integer))
  (if (`self.bIsPressed`)
    (if (== (`KismetArrayLibrary.Array_Length` (`PrimitiveComponent.GetOverlappingActors` (`self.Box`) "/Game/ThirdPerson/Blueprints/BP_ThirdPersonCharacter.BP_ThirdPersonCharacter_C")) 0)
      (set `self.bIsPressed` false)
      (`self.BroadcastOnInteracted`))))

(fn `UserConstructionScript`
  (`parent.UserConstructionScript`))