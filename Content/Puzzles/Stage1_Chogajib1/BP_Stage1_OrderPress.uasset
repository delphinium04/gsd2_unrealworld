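; BP_Stage1_OrderPress is a Stage 1 puzzle that is solved by interacting with a set of actors in a specific order.
; On BeginPlay it binds to each PressActor's OnInteracted event, treating the array order as the required sequence.
; Each correct press advances CurrentIndex, while a wrong one resets it to zero.
; Completing the sequence broadcasts OnPuzzleSolved once and unbinds the actors' interaction events.
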(event `self.ReceiveBeginPlay`
  (`parent.ReceiveBeginPlay`)
  (for _array_element (`self.PressActor`)
    (add `InteractableActor.OnInteracted` _array_element (delegate `CustomEvent`))))

(event `CustomEvent`
  (params (Caller :type "InteractableActor Object Reference"))
  (`self.Check` Caller))

(fn `Check`
  (params (Interactable :type "InteractableActor Object Reference"))
  (if (== Interactable (`|GetArrayItem` (`self.PressActor`) (`self.CurrentIndex`)))
    (bind _result (`/Engine/EditorBlueprintResources/StandardMacros.IncrementInt` (`self.CurrentIndex`))
      (:`  `
        (if (== _result (`KismetArrayLibrary.Array_Length` (`self.PressActor`)))
          (`/Engine/EditorBlueprintResources/StandardMacros.DoOnce` false
            (:`Completed`
              (`self.Solved`))))))
    (else
      (set `self.CurrentIndex` 0))))

(fn `Solved`
  (set `self.CurrentIndex` 0)
  (`self.BroadcastOnPuzzleSolved`)
  (for _array_element (`self.PressActor`)
    (clear `InteractableActor.OnInteracted` _array_element)))

(fn `UserConstructionScript`
  (`parent.UserConstructionScript`))