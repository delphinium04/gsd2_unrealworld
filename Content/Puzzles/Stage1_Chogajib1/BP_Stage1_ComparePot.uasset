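; Stage 1 puzzle actor that compares how many TargetActor instances sit in its left and right areas.
; It counts both areas at BeginPlay and recounts them from the overlapping actors on every begin or end overlap.
; After each overlap recount, equal counts broadcast OnPuzzleSolved through a DoOnce, with no minimum count required.
; Incremental WhenOverlapBegin and WhenOverlapExit counters are defined but not called in this graph.
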(event `self.ReceiveBeginPlay`
  (`parent.ReceiveBeginPlay`)
  (`self.SetDefaultCount`))

(event `self.LeftArea.OnComponentBeginOverlap`
  (params (OverlappedComponent :type "PrimitiveComponent Object Reference") (OtherActor :type "Actor Object Reference") (OtherComp :type "PrimitiveComponent Object Reference") (OtherBodyIndex :type Integer) (bFromSweep :type Boolean) (SweepResult :type "HitResult Structure (by ref)"))
  (`self.SetDefaultCount` :!label _label)
  (`self.CheckPuzzleEnd`))

(event `self.RightArea.OnComponentBeginOverlap`
  (params (OverlappedComponent :type "PrimitiveComponent Object Reference") (OtherActor :type "Actor Object Reference") (OtherComp :type "PrimitiveComponent Object Reference") (OtherBodyIndex :type Integer) (bFromSweep :type Boolean) (SweepResult :type "HitResult Structure (by ref)"))
  (goto _label))

(event `self.LeftArea.OnComponentEndOverlap`
  (params (OverlappedComponent :type "PrimitiveComponent Object Reference") (OtherActor :type "Actor Object Reference") (OtherComp :type "PrimitiveComponent Object Reference") (OtherBodyIndex :type Integer))
  (goto _label))

(event `self.RightArea.OnComponentEndOverlap`
  (params (OverlappedComponent :type "PrimitiveComponent Object Reference") (OtherActor :type "Actor Object Reference") (OtherComp :type "PrimitiveComponent Object Reference") (OtherBodyIndex :type Integer))
  (goto _label))

(fn `CheckPuzzleEnd`
  (if (== (`self.RightCount`) (`self.LeftCount`))
    (`/Engine/EditorBlueprintResources/StandardMacros.DoOnce` false
      (:`Completed`
        (`self.BroadcastOnPuzzleSolved`)))))

(fn `SetDefaultCount`
  (set `self.LeftCount` (`KismetArrayLibrary.Array_Length` (`PrimitiveComponent.GetOverlappingActors` (`self.LeftArea`) (`self.TargetActor`))))
  (set `self.RightCount` (`KismetArrayLibrary.Array_Length` (`PrimitiveComponent.GetOverlappingActors` (`self.RightArea`) (`self.TargetActor`)))))

(fn `UserConstructionScript`
  (`parent.UserConstructionScript`))

(fn `WhenOverlapBegin`
  (params (Other :type "Object Object Reference") (IsLeft :type Boolean))
  (if (== (`GameplayStatics.GetObjectClass` Other) (`self.TargetActor`))
    (if IsLeft
      (bind _result (`/Engine/EditorBlueprintResources/StandardMacros.IncrementInt` (`self.LeftCount`))
        (:`  `
          (set `self.LeftCount` _result)))
      (else
        (bind _result_2 (`/Engine/EditorBlueprintResources/StandardMacros.IncrementInt` (`self.RightCount`))
          (:`  `
            (set `self.RightCount` _result_2)))))
    (`self.CheckPuzzleEnd`)))

(fn `WhenOverlapExit`
  (params (Other :type "Object Object Reference") (IsLeft :type Boolean))
  (if (== (`GameplayStatics.GetObjectClass` Other) (`self.TargetActor`))
    (if IsLeft
      (bind _result (`/Engine/EditorBlueprintResources/StandardMacros.DecrementInt` (`self.LeftCount`))
        (:`  `
          (set `self.LeftCount` _result)))
      (else
        (bind _result_2 (`/Engine/EditorBlueprintResources/StandardMacros.DecrementInt` (`self.RightCount`))
          (:`  `
            (set `self.RightCount` _result_2)))))
    (`self.CheckPuzzleEnd`)))