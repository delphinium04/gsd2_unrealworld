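; BP_TestPuzzle is a test puzzle actor that counts as solved as soon as any of its linked objects is interacted with.
; On BeginPlay it binds one event to OnInteracted on every entry in Objects, with no condition check.
; Success broadcasts OnPuzzleSolved, clears all OnInteracted bindings on those objects and activates an auto-destroying Niagara effect.
; CheckCube1 is an unused stub returning false.
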(event `self.ReceiveBeginPlay`
  (`parent.ReceiveBeginPlay`)
  (`self.Bind` (delegate `CustomEvent`)))

(event `CustomEvent`
  (params (Caller :type "InteractableActor Object Reference"))
  (`self.OnInteractableStateChanged`))

(event `self.OnInteractableStateChanged`
  (`self.Success`))

(fn `Bind`
  (params (Delegate :type "Delegate (by ref)"))
  (for _array_element (`self.Objects`)
    (add `InteractableActor.OnInteracted` _array_element Delegate)))

(fn `CheckCube1`
  (returns (Succeed :type Boolean))
  (return false))

(fn `Success`
  (bind _niagaracomponent (`NiagaraActor.NiagaraComponent` (`self.Niagara`)))
  (`self.BroadcastOnPuzzleSolved`)
  (`self.Unbind`)
  (`ActorComponent.Activate` _niagaracomponent false)
  (`NiagaraComponent.SetAutoDestroy` _niagaracomponent true))

(fn `Unbind`
  (for _array_element (`self.Objects`)
    (clear `InteractableActor.OnInteracted` _array_element)))

(fn `UserConstructionScript`
  (`parent.UserConstructionScript`))