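; BP_StagePortal is a portal actor that opens another level when the player character overlaps its collision.
; The destination comes from the LevelName enum, whose value is converted to a name for OpenLevelByName.
; The construction script applies the Material and PortalVisibility variables to the portal's plane mesh.
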(event `self.Collision.OnComponentBeginOverlap`
  (params (OverlappedComponent :type "PrimitiveComponent Object Reference") (OtherActor :type "Actor Object Reference") (OtherComp :type "PrimitiveComponent Object Reference") (OtherBodyIndex :type Integer) (bFromSweep :type Boolean) (SweepResult :type "HitResult Structure (by ref)"))
  (cast `PlayerCharacter` OtherActor)
  (`GameplayStatics.OpenLevel` (`|GetEnumeratorName` (`self.LevelName`))))

(fn `UserConstructionScript`
  (`PrimitiveComponent.SetMaterial` (`self.SM_Plane`) 0 (`self.Material`))
  (`SceneComponent.SetVisibility` (`self.SM_Plane`) (`self.Portal Visibility`) false))