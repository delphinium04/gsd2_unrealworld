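; Pickup actor for the Unra item in the Stage 2 Jongmyo puzzle.
; Any actor overlap enables player input and sets ItemGet; ending the overlap reverses both.
; Pressing the item-pickup action then destroys the actor, plays the pickup sound at world origin and adds Unra to the first BP_QuestArena found.
; It also puts a QuestList_Unra widget on the viewport.
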(event `self.ReceiveBeginPlay`
  (`parent.ReceiveBeginPlay`))

(event `InputAction|아이템 습득`
  (params (Key :type "Key Structure"))
  (:`Pressed`
    (if (stale `self.ReceiveActorBeginOverlap` _output_get)
      (`self.K2_DestroyActor`)
      (`GameplayStatics.PlaySoundAtLocation` "/Game/Naganeupseong/Quest_Item/PickUp.PickUp" (0.0 0.0 0.0) (struct) 1.0 1.0 0.0 null null null null)
      (bind _outactors (`GameplayStatics.GetAllActorsOfClass` "/Game/Puzzles/Stage2_Jongmyo/BP_QuestArena.BP_QuestArena_C"))
      (`/Game/Puzzles/Stage2_Jongmyo/BP_QuestArena.AddItem` (`|GetArrayItem` _outactors) (`self.Unra`))
      (bind _returnvalue (`|CreateWidget` "/Game/Jongmyo/Stage2_Text/QuestList_Unra.QuestList_Unra_C"))
      (`UserWidget.AddToViewport` _returnvalue 0))))

(event `self.ReceiveActorBeginOverlap`
  (params (OtherActor :type "Actor Object Reference"))
  (`parent.ReceiveActorBeginOverlap` OtherActor)
  (`self.EnableInput` (`GameplayStatics.GetPlayerController` 0))
  (bind _output_get (set `self.bItemGet` true)))

(event `self.ReceiveActorEndOverlap`
  (params (OtherActor :type "Actor Object Reference"))
  (`self.DisableInput` (`GameplayStatics.GetPlayerController` 0))
  (set `self.bItemGet` false))

(fn `UserConstructionScript`
  (`parent.UserConstructionScript`))