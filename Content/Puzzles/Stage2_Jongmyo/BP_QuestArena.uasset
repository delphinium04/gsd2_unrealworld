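; BP_QuestArena is the table in the Stage 2 Jongmyo puzzle that checks whether the main quest instruments are collected.
; Overlap enables input and sets a Quest flag, letting the item-pickup action run HasAllItem against six traditional Korean instruments.
; HasAllItem searches CollectedItem, filled through AddItem.
; A full set destroys the actor and triggers CallStageClear; otherwise, it shows the Stage2_QuestFalse widget.
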(event `self.ReceiveBeginPlay`
  (`parent.ReceiveBeginPlay`))

(event `InputAction|아이템 습득`
  (params (Key :type "Key Structure"))
  ; 밥상에 다가가서 E키를 누르면 메인 퀘스트 아이템 수집 여부 확인
  (:`Pressed`
    (if (stale `self.ReceiveActorBeginOverlap` _output_get)
      (bind _stageclear (`self.HasAllItem` (`|MakeArray` (`self.Gayageum`) (`self.Janggu`) (`self.Jeolgo`) (`self.Unra`) (`self.Daegeum`) (`self.Nagak`))))
      (if _stageclear
        (`self.StageClear`)))))

(event `self.ReceiveActorBeginOverlap`
  (params (OtherActor :type "Actor Object Reference"))
  ; 밥상에 다가가서 E키를 누르면 메인 퀘스트 아이템 수집 여부 확인
  (`parent.ReceiveActorBeginOverlap` OtherActor)
  (`self.EnableInput` (`GameplayStatics.GetPlayerController` 0))
  (bind _output_get (set `self.Quest` true)))

(event `self.ReceiveActorEndOverlap`
  (params (OtherActor :type "Actor Object Reference"))
  ; 밥상에 다가가서 E키를 누르면 메인 퀘스트 아이템 수집 여부 확인
  (set `self.Quest` false))

(fn `AddItem`
  (params (ItemType :type String))
  (bind _output_get (set `self.ItemType` ItemType))
  (`KismetArrayLibrary.Array_Add` (`self.CollectedItem`) _output_get))

(fn `HasAllItem`
  (params (QuestItem :type "Array of String"))
  (returns (StageClear :type Boolean))
  ; 메인 퀘스트 클리어 여부 판단
  (set `self.FoundAllItem` true)
  (for _array_element QuestItem
    (if (not (`KismetArrayLibrary.Array_Contains` (`self.CollectedItem`) _array_element))
      (set `self.FoundAllItem` false)))
  (if (`self.FoundAllItem`)
    (`self.K2_DestroyActor`)
    (return true)
    (else
      (bind _returnvalue (`|CreateWidget` "/Game/Jongmyo/Stage2_Text/Stage2_QuestFalse.Stage2_QuestFalse_C"))
      (`UserWidget.AddToViewport` _returnvalue 0))))

(fn `UserConstructionScript`
  (`parent.UserConstructionScript`))