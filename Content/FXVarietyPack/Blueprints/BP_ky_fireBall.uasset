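; BP_ky_fireBall is a fireball projectile effect that spawns a color-tinted shockwave on BeginPlay and flies along its local X axis.
; Tick counts down its lifetime and moves it by speed, scaled by a timeline-driven correction curve.
; A polling delay loop started from the timeline update disables collision, fades the FX and destroys it on expiry.
; Overlapping an actor whose first tag isn't "ky_shot" spawns a hit effect and destroys it immediately.
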(event `self.ReceiveBeginPlay`
  (bind _defaultsceneroot (`self.DefaultSceneRoot`))
  ;[1 1 1] 파이어볼 등장시 시각 효과 생성
  (bind _returnvalue (`GameplayStatics.SpawnEmitterAtLocation` "/Game/FXVarietyPack/Particles/P_ky_shotShockwave.P_ky_shotShockwave" (`SceneComponent.K2_GetComponentLocation` _defaultsceneroot) (`SceneComponent.K2_GetComponentRotation` _defaultsceneroot)))
  (`ParticleSystemComponent.SetVectorParameter` _returnvalue "color" (`KismetMathLibrary.Conv_LinearColorToVector` (`self.color`)))
  ;[1 1 1] 이펙트가 제대로 갈 수 있도록
  (bind (_direction _valuecorrect) (`Timeline|Timeline_0`)
    (:`Update`
      (set `self.speedCorrect` _valuecorrect)
      ;[1 1 1] 지속 시간 판단
      (`KismetSystemLibrary.Delay` 0.1 :!label _label)
      (if (< (`self.duration`) 0.0)
        ;[1 1 1] 충돌 후 시각 효과 파괴
        (`PrimitiveComponent.SetCollisionEnabled` (`self.Box`) "NoCollision")
        (`ActorComponent.Deactivate` (`self.FX1`))
        (`KismetSystemLibrary.Delay` 1.0)
        ;[1 1 1] effect destroy
        (`self.K2_DestroyActor`)
        (else
          (goto _label))))))

(event `self.ReceiveTick`
  (params (DeltaSeconds :type "Float (single-precision)"))
  ;[1 1 1] 이동과 거리 제어
  (set `self.duration` (- (`self.duration`) DeltaSeconds))
  ;[1 1 1] 이동
  (`self.K2_AddActorLocalOffset` (`KismetMathLibrary.MakeVector` (* (`self.speed`) (`self.speedCorrect`) (`GameplayStatics.GetWorldDeltaSeconds`)))))

(event `self.ReceiveActorBeginOverlap`
  (params (OtherActor :type "Actor Object Reference"))
  ;[1 1 1] 충돌 시 이펙트
  (if (`KismetSystemLibrary.IsValid` OtherActor)
    (if (!= (`|GetArrayItem` (`Actor.Tags` OtherActor)) "ky_shot")
      (`GameplayStatics.SpawnEmitterAtLocation` (`self.hitFx`) (`SceneComponent.K2_GetComponentLocation` (`self.Box`)))
      ;[1 1 1] 자신 제거
      (`self.K2_DestroyActor`))))

(fn `UserConstructionScript`)