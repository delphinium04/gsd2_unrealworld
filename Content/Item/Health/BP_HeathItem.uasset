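; BP_HeathItem is a health pickup actor with Niagara effects, though healing is so far only a debug print.
; The first sphere overlap from any actor, gated by DoOnce, prints the heal message, deactivates the auto-activated root effect and activates the interaction effect.
; The actor destroys itself when that interaction effect finishes, through a delegate bound on BeginPlay.
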(event `self.ReceiveBeginPlay`
  (add `NiagaraComponent.OnSystemFinished` (`self.NiagaraInteraction`) (delegate `OnSystemFinished_Event`)))

(event `OnSystemFinished_Event`
  (params (PSystem :type "NiagaraComponent Object Reference"))
  (`self.K2_DestroyActor`))

(event `self.SphereComponent.OnComponentBeginOverlap`
  (params (OverlappedComponent :type "PrimitiveComponent Object Reference") (OtherActor :type "Actor Object Reference") (OtherComp :type "PrimitiveComponent Object Reference") (OtherBodyIndex :type Integer) (bFromSweep :type Boolean) (SweepResult :type "HitResult Structure (by ref)"))
  (`/Engine/EditorBlueprintResources/StandardMacros.DoOnce` false
    (:`Completed`
      (`self.OnOverlapWithPlayer`))))

(event `self.OnOverlapWithPlayer`
  (`KismetSystemLibrary.PrintString` "Send HealMessage to player")
  (`ActorComponent.Deactivate` (`self.NiagaraRoot`))
  (`ActorComponent.Activate` (`self.NiagaraInteraction`) false))

(fn `UserConstructionScript`
  (`parent.UserConstructionScript`)
  (`ActorComponent.SetAutoActivate` (`self.NiagaraRoot`) true))