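; BP_Rice is a rice quest-item pickup that the player collects with the item pickup input action.
; Sphere overlap enables player 0's input, sets ItemGet and shows a widget hidden at BeginPlay; end overlap reverses this, and neither checks which actor overlapped.
; Pressing the action while ItemGet is set destroys the actor, plays the PickUp sound at world origin and adds Rice1 to the first BP_QuestTable found.
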(event `self.ReceiveBeginPlay`
  (`SceneComponent.SetVisibility` (`self.Widget`) false false))

(event `InputAction|아이템 습득`
  (params (Key :type "Key Structure"))
  (:`Pressed`
    (if (stale `self.Sphere.OnComponentBeginOverlap` _output_get)
      (`self.K2_DestroyActor`)
      (`GameplayStatics.PlaySoundAtLocation` "/Game/Naganeupseong/Quest_Item/PickUp.PickUp" (0.0 0.0 0.0) (struct) 1.0 1.0 0.0 null null null null)
      (bind _outactors (`GameplayStatics.GetAllActorsOfClass` "/Game/Puzzles/Stage1_Chogajib1/BP_QuestTable.BP_QuestTable_C"))
      (`/Game/Puzzles/Stage1_Chogajib1/BP_QuestTable.AddItem` (`|GetArrayItem` _outactors) (`self.Rice1`)))))

(event `self.Sphere.OnComponentBeginOverlap`
  (params (OverlappedComponent :type "PrimitiveComponent Object Reference") (OtherActor :type "Actor Object Reference") (OtherComp :type "PrimitiveComponent Object Reference") (OtherBodyIndex :type Integer) (bFromSweep :type Boolean) (SweepResult :type "HitResult Structure (by ref)"))
  (`self.EnableInput` (`GameplayStatics.GetPlayerController` 0))
  (bind _output_get (set `self.bItemGet` true))
  (`SceneComponent.SetVisibility` (`self.Widget`) true false))

(event `self.Sphere.OnComponentEndOverlap`
  (params (OverlappedComponent :type "PrimitiveComponent Object Reference") (OtherActor :type "Actor Object Reference") (OtherComp :type "PrimitiveComponent Object Reference") (OtherBodyIndex :type Integer))
  (`self.DisableInput` (`GameplayStatics.GetPlayerController` 0))
  (`SceneComponent.SetVisibility` (`self.Widget`) false false)
  (set `self.bItemGet` false))

(fn `UserConstructionScript`)