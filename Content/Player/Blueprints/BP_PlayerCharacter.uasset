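; Player character Blueprint that carries a weapon and tracks health shown on a gameplay widget.
; BeginPlay spawns a weapon onto the mesh's weapon socket, creates the UI and fills health to maximum.
; J and K step health down or up within limits and refresh the UI, with J calling Die at zero.
; AnyDamage subtracts truncated damage without refreshing the UI, and at zero plays a death montage before destroying the actor.
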(event `self.ReceiveBeginPlay`
  (bind _w_gameplay (`self.W_GamePlay`))
  (bind _returnvalue (`|SpawnActorFromClass` "/Game/Player/Blueprints/BP_Weapon.BP_Weapon_C" (`self.GetTransform`) "Undefined" "MultiplyWithRoot" null null))
  (bind _output_get (set `self.WeaponActor` _returnvalue))
  (`self.K2_AttachToComponent` _output_get (`self.Mesh`) "weapon_socket" "SnapToTarget" "SnapToTarget" "SnapToTarget" true)
  (bind _returnvalue_2 (`|CreateWidget` "/Game/Player/Blueprints/GamePlayUi.GamePlayUi_C" (`GameplayStatics.GetPlayerController` 0)))
  (set `self.W_GamePlay` _returnvalue_2)
  (set `self.CurrentHealth_0` (`self.MaxHealth`))
  (`UserWidget.AddToViewport` _w_gameplay 0)
  (`/Game/Player/Blueprints/GamePlayUi.Set Health` _w_gameplay (`self.CurrentHealth_0`) (`self.MaxHealth`)))

(event `Key|J`
  (params (Key :type "Key Structure"))
  (bind _currenthealth_0 (`self.CurrentHealth_0`))
  (:`Pressed`
    (set `self.CurrentHealth_0` (`KismetMathLibrary.Max` 0 (- (`self.CurrentHealth_0`) 1)))
    (`/Game/Player/Blueprints/GamePlayUi.Set Health` (`self.W_GamePlay`) _currenthealth_0 (`self.MaxHealth`))
    (if (<= _currenthealth_0 0)
      (`self.Die`))))

(event `Key|K`
  (params (Key :type "Key Structure"))
  (:`Pressed`
    (set `self.CurrentHealth_0` (`KismetMathLibrary.Min` (`self.MaxHealth`) (+ (`self.CurrentHealth_0`) 1)))
    (`/Game/Player/Blueprints/GamePlayUi.Set Health` (`self.W_GamePlay`) (`self.CurrentHealth_0`) (`self.MaxHealth`))))

(event `self.ReceiveAnyDamage`
  (params (Damage :type "Float (single-precision)") (DamageType :type "DamageType Object Reference") (InstigatedBy :type "Controller Object Reference") (DamageCauser :type "Actor Object Reference"))
  (bind _output_get (set `self.CurrentHealth_0` (`KismetMathLibrary.FTrunc` (- (`self.CurrentHealth_0`) Damage))))
  (if (<= _output_get 0)
    (`|PlayMontage` null "/Game/Player/Montage/Death_Montage.Death_Montage"
      (:`OnCompleted`
        (`self.K2_DestroyActor`)))))

(fn `UserConstructionScript`)